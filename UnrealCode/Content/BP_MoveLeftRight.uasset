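; BP_MoveLeftRight is an actor whose static mesh slides back and forth along relative X while activated by a linked Switch.
; BeginPlay binds to the Switch's overlap dispatcher, or prints an error if none is assigned.
; EventOverlap sets IsPlay from the overlap begin state.
; While playing, Tick moves the mesh a fixed step per frame, independent of delta time, flipping direction at each end of its range.
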(event EventBeginPlay
  (bind _switch (Variables|Default|GetSwitch))
  (Utilities|IsValid _switch
    (:Is%20Valid
      ;[1 1 1] 이벤트에 바인딩(이벤트를 팔로우한다)
      (EventDispatchers|BindEventtoEventDispatcherOverlap _switch (EventDispatchers|CreateEvent :!event EventOverlap)))
    (:Is%20Not%20Valid
      (Development|PrintString "디테일 스위치 객체 정보안넣음" true true "(R=1.000000,G=0.000000,B=0.113355,A=1.000000)" 2e+01))))

(event EventTick
  (params (DeltaSeconds :type Float%20%28single-precision%29))
  (if (Variables|Default|GetIsPlay)
    (if (Variables|Default|Getright_)
      ;[1 1 1] 오른쪽 이동
      (bind _output_get (Variables|Default|Settran_x (+ (Variables|Default|Gettran_x) 1.0)))
      (Transformation|SetRelativeLocation (Variables|Default|GetStaticMesh) (Math|Vector|MakeVector _output_get 0.0 0.0) false false)
      (if (>= (Variables|Default|Gettran_x) 1e+02)
        (Variables|Default|Setright_ false))
      (else
        ;[1 1 1] 왼쪽쪽 이동
        (bind _output_get_2 (Variables|Default|Settran_x (+ (Variables|Default|Gettran_x) -1.0)))
        (Transformation|SetRelativeLocation (Variables|Default|GetStaticMesh) (Math|Vector|MakeVector _output_get_2 0.0 0.0) false false)
        (if (<= (Variables|Default|Gettran_x) 0.0)
          (Variables|Default|Setright_ true))))))

(fn ConstructionScript)

(fn EventOverlap
  (params (IsBegin :type Boolean))
  (Variables|Default|SetIsPlay IsBegin))

(fn 새함수
  (params (IsPlay :type Boolean))
  (Variables|Default|SetIsPlay IsPlay)
  (return false))